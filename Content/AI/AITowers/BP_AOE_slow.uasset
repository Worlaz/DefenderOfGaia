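; Area-of-effect tower actor that slows BP_Parent_Enemy_NPC enemies overlapping its CollisionComponent.
; Begin overlap multiplies the enemy's SpeedChange by SlowEffect unless that breaches MinSpeedChangeCap, then always multiplies current MaxWalkSpeed by SpeedChange.
; End overlap divides SpeedChange by SlowEffect, even if the cap blocked the slow, and again multiplies current MaxWalkSpeed by it.
; Walk speed therefore compounds rather than being recomputed from a stored base.
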(event `self.ReceiveTick`
  (params (DeltaSeconds :type "Float (single-precision)")))

(event `self.CollisionComponent.OnComponentBeginOverlap`
  (params (OverlappedComponent :type "PrimitiveComponent Object Reference") (OtherActor :type "Actor Object Reference") (OtherComp :type "PrimitiveComponent Object Reference") (OtherBodyIndex :type Integer) (bFromSweep :type Boolean) (SweepResult :type "HitResult Structure (by ref)"))
  ;[1 1 1] If Overlap Actor is a child of NPC_parent, slow their speed
  (if (`KismetMathLibrary.ClassIsChildOf` (`GameplayStatics.GetObjectClass` OtherActor) "/Game/AI/NPC/ModifiedNPC/BP_Parent_Enemy_NPC.BP_Parent_Enemy_NPC_C")
    (bind _asbp_parent_enemy_npc (cast `/Game/AI/NPC/ModifiedNPC/BP_Parent_Enemy_NPC` OtherActor))
    (bind _returnvalue (* (`/Game/AI/NPC/ModifiedNPC/BP_Parent_Enemy_NPC.SpeedChange` _asbp_parent_enemy_npc) (`self.SlowEffect`)))
    ;[1 1 1] Apply slow to variables stored in the NPC, until a set threshold is reached
    (if (>= _returnvalue (`/Game/AI/NPC/ModifiedNPC/BP_Parent_Enemy_NPC.MinSpeedChangeCap` _asbp_parent_enemy_npc))
      (bind _output_get (set `/Game/AI/NPC/ModifiedNPC/BP_Parent_Enemy_NPC.SpeedChange` _returnvalue _asbp_parent_enemy_npc)))
    (bind _charactermovement (`Character.CharacterMovement` _asbp_parent_enemy_npc))
    (set `CharacterMovementComponent.MaxWalkSpeed` (* _output_get (`CharacterMovementComponent.MaxWalkSpeed` _charactermovement)) _charactermovement)))

(event `self.CollisionComponent.OnComponentEndOverlap`
  (params (OverlappedComponent :type "PrimitiveComponent Object Reference") (OtherActor :type "Actor Object Reference") (OtherComp :type "PrimitiveComponent Object Reference") (OtherBodyIndex :type Integer))
  ;[1 1 1] When Overlap ends and the actor is a child of NPC_parent remove slow effect
  (if (`KismetMathLibrary.ClassIsChildOf` (`GameplayStatics.GetObjectClass` OtherActor) "/Game/AI/NPC/ModifiedNPC/BP_Parent_Enemy_NPC.BP_Parent_Enemy_NPC_C")
    (bind _asbp_parent_enemy_npc (cast `/Game/AI/NPC/ModifiedNPC/BP_Parent_Enemy_NPC` OtherActor))
    (bind _output_get (set `/Game/AI/NPC/ModifiedNPC/BP_Parent_Enemy_NPC.SpeedChange` (/ (`/Game/AI/NPC/ModifiedNPC/BP_Parent_Enemy_NPC.SpeedChange` _asbp_parent_enemy_npc) (`self.SlowEffect`)) _asbp_parent_enemy_npc))
    (bind _charactermovement (`Character.CharacterMovement` _asbp_parent_enemy_npc))
    (set `CharacterMovementComponent.MaxWalkSpeed` (* _output_get (`CharacterMovementComponent.MaxWalkSpeed` _charactermovement)) _charactermovement)))

(fn `UserConstructionScript`)