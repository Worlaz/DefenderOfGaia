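; Automated turret that finds enemy NPCs within attack range and shoots homing projectiles at them.
; Each tick without a target, it scans all BP_Parent_Enemy_NPC actors and locks onto the first in range until it becomes invalid or leaves.
; The crystal smoothly turns toward the target on yaw only.
; Firing is called every tick, with a Delay throttling projectile spawns at the Barrel socket to the fire interval.
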(event `self.ReceiveTick`
  (params (DeltaSeconds :type "Float (single-precision)"))
  (set `self.DeltaTime` DeltaSeconds)
  (`self.UpdateRotation`)
  (`self.FireProjectile` (0.0 0.0 0.0)))

(event `UpdateRotation`
  (bind _output (`|GetArrayItem` (`self.NPC_Mesh2`) (`self.NPCIndex`)))
  (if (`self.EnemyInRange`)
    (bind _isinrange (`self.CalculateInRange` _output))
    (if _isinrange
      (`/Engine/EditorBlueprintResources/StandardMacros.IsValid` _output :!label _label
        (:`Is Valid`
          (`SceneComponent.K2_SetWorldRotation` (`self.TurretCrystal`) (`KismetMathLibrary.RInterpTo` (`SceneComponent.K2_GetComponentRotation` (`self.TurretCrystal`)) (`KismetMathLibrary.MakeRotator` 0.0 0.0 (.yaw (`KismetMathLibrary.FindLookAtRotation` (`SceneComponent.K2_GetComponentLocation` (`self.DefaultSceneRoot`)) (`SceneComponent.K2_GetComponentLocation` (`Actor.RootComponent` _output))))) (`self.DeltaTime`) (`self.RotationSpeed`)) false false))
        (:`Is Not Valid`
          (set `self.EnemyInRange` false)))
      (else
        (set `self.EnemyInRange` false)))
    (else
      (bind _outactors (`GameplayStatics.GetAllActorsOfClass` "/Game/AI/NPC/ModifiedNPC/BP_Parent_Enemy_NPC.BP_Parent_Enemy_NPC_C"))
      (bind _output_get (set `self.NPC_Mesh2` _outactors))
      (if (> (`KismetArrayLibrary.Array_Length` _output_get) 0)
        (for (_array_element _array_index) _output_get
          (`/Engine/EditorBlueprintResources/StandardMacros.IsValid` _array_element
            (:`Is Valid`
              (set `self.NPCIndex` _array_index)
              (bind _isinrange_2 (`self.CalculateInRange` _array_element))
              (bind _output_get_2 (set `self.EnemyInRange` _isinrange_2))
              (if _output_get_2
                (break)))))
        (if (`self.EnemyInRange`)
          (goto _label))))))

(event `FireProjectile`
  (params (TargetPosition :type "Vector Structure"))
  (bind _output (`|GetArrayItem` (`self.NPC_Mesh2`) (`self.NPCIndex`)))
  ;[1 1 1] Fire projectile
  (if (`self.EnemyInRange`)
    (`/Engine/EditorBlueprintResources/StandardMacros.IsValid` _output
      (:`Is Valid`
        (`KismetSystemLibrary.Delay` (`self.FireInterval`))
        (bind _returnvalue (`|SpawnActorFromClass` "/Game/AI/AI_turret/BP_Turret_Projectile.BP_Turret_Projectile_C" (`SceneComponent.GetSocketTransform` (`self.TurretCrystal`) "Barrel" "RTS_World") "Undefined" "OverrideRootScale" null null))
        (`/Game/AI/AI_turret/BP_Turret_Projectile.SetHomingTarget` _returnvalue _output)))))

(fn `CalculateInRange`
  (params (NPC_Enemy :type "/Game/AI/NPC/ModifiedNPC/BP_Parent_Enemy_NPC Object Reference (by ref)"))
  (returns (IsInRange :type Boolean))
  (bind _returnvalue (< (`KismetMathLibrary.VSize` (- (`SceneComponent.K2_GetComponentLocation` (`self.DefaultSceneRoot`)) (`SceneComponent.K2_GetComponentLocation` (`Actor.RootComponent` NPC_Enemy)))) (`self.AttackRange`)))
  (if _returnvalue
    _
    (else
      _))
  (return _returnvalue))

(fn `UserConstructionScript`)