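; Parent Blueprint for enemy NPCs with an overhead health bar widget that can be destroyed by projectile hits.
; BeginPlay seeds the WG_NPC_HealthBar with StartHealth, and Tick rotates the bar from the player controller's rotation to face the camera.
; Capsule overlaps with "Projectile"-tagged actors destroy the projectile and copy CurrentHealth to the widget, destroying the NPC at zero or below.
; No damage subtraction happens in this graph.
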(event `self.ReceiveBeginPlay`
  (bind _start_health (`self.Start_Health`))
  (bind _aswg_npc_health_bar (cast `/Game/AI/NPC/WG_NPC_HealthBar` (`WidgetComponent.GetUserWidgetObject` (`self.HealthBar`))))
  (set `/Game/AI/NPC/WG_NPC_HealthBar.StartHealth` _start_health _aswg_npc_health_bar)
  (set `/Game/AI/NPC/WG_NPC_HealthBar.CurrentHealth` _start_health _aswg_npc_health_bar))

(event `self.ReceiveTick`
  (params (DeltaSeconds :type "Float (single-precision)"))
  (bind _healthbar (`self.HealthBar`))
  ;[1 1 1] Make the HealthBar Widget always face the camera
  (`SceneComponent.K2_SetWorldRotation` _healthbar (.rotation (`self.GetTransform` (`GameplayStatics.GetPlayerController` 0))) false false)
  (`SceneComponent.K2_AddLocalRotation` _healthbar (struct :`Yaw` -180.0) false false))

(event `self.CapsuleComponent.OnComponentBeginOverlap`
  (params (OverlappedComponent :type "PrimitiveComponent Object Reference") (OtherActor :type "Actor Object Reference") (OtherComp :type "PrimitiveComponent Object Reference") (OtherBodyIndex :type Integer) (bFromSweep :type Boolean) (SweepResult :type "HitResult Structure (by ref)"))
  ;[1 1 1] Based on "Tag" check if we have been hit
  (if (`self.ActorHasTag` OtherActor "Projectile")
    (`self.K2_DestroyActor` OtherActor)
    (`KismetSystemLibrary.PrintString` "WE GOT HIT")
    (bind _aswg_npc_health_bar (cast `/Game/AI/NPC/WG_NPC_HealthBar` (`WidgetComponent.GetUserWidgetObject` (`self.HealthBar`))))
    (bind _output_get (set `/Game/AI/NPC/WG_NPC_HealthBar.CurrentHealth` (`self.Current_Health`) _aswg_npc_health_bar))
    (if (<= _output_get 0.0)
      (`self.K2_DestroyActor`))))

(event `self.Mesh.OnComponentBeginOverlap`
  (params (OverlappedComponent :type "PrimitiveComponent Object Reference") (OtherActor :type "Actor Object Reference") (OtherComp :type "PrimitiveComponent Object Reference") (OtherBodyIndex :type Integer) (bFromSweep :type Boolean) (SweepResult :type "HitResult Structure (by ref)")))

(fn `UserConstructionScript`)