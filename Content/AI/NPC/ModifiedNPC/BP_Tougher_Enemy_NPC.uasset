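; Tougher enemy NPC Blueprint with a melee attack that damages the first-person player character.
; MeleeAttack plays the attack montage, followed shortly by a miss sound at the capsule's location.
; A collision component, attached to the right-hand socket in the construction script, applies damage on overlap while AttackReady is set.
; A DoOnce gate with a delayed reset prevents repeated hits, and each hit prints a debug damage message.
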(event `/Game/AI/NPC/AI_CombatInterface.Melee Attack`
  (`|PlayMontage` (`self.Mesh`) "/Game/AI/NPC/ModifiedNPC/Melee_Attack_Montage.Melee_Attack_Montage"
    (:`then`
      (`KismetSystemLibrary.Delay` 0.1)
      (`GameplayStatics.PlaySoundAtLocation` "/Game/SoundEffects/MeleeMiss_Cue.MeleeMiss_Cue" (`SceneComponent.K2_GetComponentLocation` (`self.CapsuleComponent`)) (struct) 1.0 1.0 0.0 null null null))))

(event `self.RightHandCollision.OnComponentBeginOverlap`
  (params (OverlappedComponent :type "PrimitiveComponent Object Reference") (OtherActor :type "Actor Object Reference") (OtherComp :type "PrimitiveComponent Object Reference") (OtherBodyIndex :type Integer) (bFromSweep :type Boolean) (SweepResult :type "HitResult Structure (by ref)"))
  ;[1 1 1] Deal Damage
  (bind _asfirst_person_character (cast `/Game/FirstPersonBP/Blueprints/FirstPersonCharacter` OtherActor))
  (if (`self.AttackReady`)
    (`/Engine/EditorBlueprintResources/StandardMacros.DoOnce` false :!label _label
      (:`Completed`
        (bind _returnvalue (`GameplayStatics.ApplyDamage` _asfirst_person_character (`self.AttackDamage`)))
        (`KismetSystemLibrary.PrintString` (`KismetStringLibrary.Concat_StrStr` "Damage to player: " (`KismetStringLibrary.Conv_DoubleToString` _returnvalue)))
        (`KismetSystemLibrary.Delay` 0.4)
        (goto _label :!via `Reset`)))))

(fn `UserConstructionScript`
  (`parent.UserConstructionScript`)
  (`SceneComponent.K2_AttachToComponent` (`self.RightHandCollision`) (`self.Mesh`) "hand_r" "KeepRelative" "KeepRelative" "KeepRelative" true))