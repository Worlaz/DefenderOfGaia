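; BP_Delay_StoneLarge is a gathering pickup that the player collects by holding E while in range.
; The construction script loads its item data and mesh from a data table row.
; Collider overlap toggles the nameplate, input and a gate that E presses pass through.
; A retriggerable delay adds the item and destroys the actor if E is held when it ends, while a timer polled recursively feeds the progress bar.
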(event `self.ReceiveBeginPlay`
  (bind _aswg_pickup (cast `/Game/GatheringSystem/Interactables/WG_Pickup` (`WidgetComponent.GetUserWidgetObject` (`self.Nameplate`))))
  (`TextBlock.SetText` (`/Game/GatheringSystem/Interactables/WG_Pickup.NameText` _aswg_pickup) (`KismetTextLibrary.Conv_StringToText` (`KismetStringLibrary.Concat_StrStr` "Hold [E] " (`KismetStringLibrary.Conv_NameToString` (`.Name_2_F55F729042409F7AB1EC649D09A4B562` (break `/Game/GatheringSystem/Inventory/Structures/ST_Item` (`self.Information`)))))))
  (set `/Game/GatheringSystem/Interactables/WG_Pickup.MaxTimeHeld` (`self.MaxHoldTime`) _aswg_pickup))

(event `self.InteractionCollider.OnComponentBeginOverlap`
  (params (OverlappedComponent :type "PrimitiveComponent Object Reference") (OtherActor :type "Actor Object Reference") (OtherComp :type "PrimitiveComponent Object Reference") (OtherBodyIndex :type Integer) (bFromSweep :type Boolean) (SweepResult :type "HitResult Structure (by ref)"))
  (if (`KismetMathLibrary.ClassIsChildOf` (`GameplayStatics.GetObjectClass` OtherActor) "/Game/FirstPersonBP/Blueprints/FirstPersonCharacter.FirstPersonCharacter_C")
    (`SceneComponent.SetVisibility` (`self.Nameplate`) true false)
    (`self.EnableInput` (`GameplayStatics.GetPlayerController` 0))
    (goto _label :!via `Open`)))

(event `self.InteractionCollider.OnComponentEndOverlap`
  (params (OverlappedComponent :type "PrimitiveComponent Object Reference") (OtherActor :type "Actor Object Reference") (OtherComp :type "PrimitiveComponent Object Reference") (OtherBodyIndex :type Integer))
  (if (`KismetMathLibrary.ClassIsChildOf` (`GameplayStatics.GetObjectClass` OtherActor) "/Game/FirstPersonBP/Blueprints/FirstPersonCharacter.FirstPersonCharacter_C")
    (`SceneComponent.SetVisibility` (`self.Nameplate`) false false)
    (`self.DisableInput` (`GameplayStatics.GetPlayerController` 0))
    (goto _label :!via `Close`)))

(event `StopTimer`
  (`KismetSystemLibrary.K2_PauseTimerHandle` (stale `Timer` _returnvalue)))

(event `Timer`
  (bind _returnvalue (`KismetSystemLibrary.K2_SetTimerDelegate` (delegate `Timer`) (`self.MaxHoldTime`))))

(event `Key|E`
  (params (Key :type "Key Structure"))
  (:`Pressed`
    ;[1 1 1] Set bool to check if "E" is being held
    (set `self.IsHeld` true)
    (bind _aswg_pickup (cast `/Game/GatheringSystem/Interactables/WG_Pickup` (`WidgetComponent.GetUserWidgetObject` (`self.Nameplate`))))
    (bind _nameplateprogressbar (`/Game/GatheringSystem/Interactables/WG_Pickup.NameplateProgressBar` _aswg_pickup))
    (`Widget.SetVisibility` _nameplateprogressbar "Visible")
    ;[1 1 1] When E is pressed check if we also are in range -> then show progressbar
    (`/Engine/EditorBlueprintResources/StandardMacros.Gate` true :!label _label
      (:`Exit`
        (`|ExecutionSequence`
          (:`then_0`
            (`KismetSystemLibrary.RetriggerableDelay` (`self.MaxHoldTime`))
            (if (`self.IsHeld`)
              (`/Game/GatheringSystem/Inventory/Libraries/BPFL_Inventory.Additem` (`self.Information`) (`.Quantity_17_3D2A65554277D23490ABBAA41E9C4759` (break `/Game/GatheringSystem/Inventory/Structures/ST_Item` (`self.Information`))))
              (`self.K2_DestroyActor`)))
          (:`then_1`
            (`self.Timer`)
            (`self.UpdateTimer`))))))
  (:`Released`
    (set `self.IsHeld` false)
    (`Widget.SetVisibility` _nameplateprogressbar "Hidden")))

(event `UpdateTimer`
  (if (`self.IsHeld`)
    (bind _aswg_pickup (cast `/Game/GatheringSystem/Interactables/WG_Pickup` (`WidgetComponent.GetUserWidgetObject` (`self.Nameplate`))))
    (set `/Game/GatheringSystem/Interactables/WG_Pickup.TimeHeld` (`KismetSystemLibrary.K2_GetTimerElapsedTimeHandle` (stale `Timer` _returnvalue)) _aswg_pickup)
    (`KismetSystemLibrary.Delay` 0.1)
    (`self.UpdateTimer`)
    (else
      (`self.StopTimer`)
      (bind _aswg_pickup_2 (cast `/Game/GatheringSystem/Interactables/WG_Pickup` (`WidgetComponent.GetUserWidgetObject` (`self.Nameplate`))))
      (set `/Game/GatheringSystem/Interactables/WG_Pickup.TimeHeld` 0.0 _aswg_pickup_2))))

(fn `UserConstructionScript`
  (bind (_datatable _rowname) (break `DataTableRowHandle` (`self.Item`)))
  ;[1 1 1] Get the ST_Item structure that corresponds with the row specified in the "item" variable, and assign it to our "information" variable
  (bind _returnvalue (`|GetDataTableRow` _datatable _rowname)
    (:`then`
      (set `self.Information` _returnvalue)
      ;[1 1 1] Update the mesh to whatever is defined in our "information" variable
      (`StaticMeshComponent.SetStaticMesh` (`self.Model`) (`.Model_14_F200B76E4885986D5143F39F95BC4A80` (break `/Game/GatheringSystem/Inventory/Structures/ST_Item` (`self.Information`)))))))