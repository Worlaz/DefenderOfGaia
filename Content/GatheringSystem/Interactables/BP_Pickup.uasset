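; BP_Pickup is a gatherable world item whose data and mesh come from a data table row.
; The construction script copies the chosen row into Information and applies its model.
; Overlap with the FirstPersonCharacter toggles an "[E] Name" nameplate and the actor's own input.
; Pressing E passes the item and quantity to Additem, destroying the pickup only if that succeeds.
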(event `self.ReceiveBeginPlay`
  (bind _aswg_pickup_nameplate (cast `/Game/GatheringSystem/Interactables/WG_Pickup_Nameplate` (`WidgetComponent.GetUserWidgetObject` (`self.Nameplate`))))
  (`TextBlock.SetText` (`/Game/GatheringSystem/Interactables/WG_Pickup_Nameplate.NameText` _aswg_pickup_nameplate) (`KismetTextLibrary.Conv_StringToText` (`KismetStringLibrary.Concat_StrStr` "[E]" (`KismetStringLibrary.Conv_NameToString` (`.Name_2_F55F729042409F7AB1EC649D09A4B562` (break `/Game/GatheringSystem/Inventory/Structures/ST_Item` (`self.Information`))))))))

(event `self.InteractionCollider.OnComponentBeginOverlap`
  (params (OverlappedComponent :type "PrimitiveComponent Object Reference") (OtherActor :type "Actor Object Reference") (OtherComp :type "PrimitiveComponent Object Reference") (OtherBodyIndex :type Integer) (bFromSweep :type Boolean) (SweepResult :type "HitResult Structure (by ref)"))
  (if (`KismetMathLibrary.ClassIsChildOf` (`GameplayStatics.GetObjectClass` OtherActor) "/Game/FirstPersonBP/Blueprints/FirstPersonCharacter.FirstPersonCharacter_C")
    (`SceneComponent.SetVisibility` (`self.Nameplate`) true false)
    (`self.EnableInput` (`GameplayStatics.GetPlayerController` 0))))

(event `self.InteractionCollider.OnComponentEndOverlap`
  (params (OverlappedComponent :type "PrimitiveComponent Object Reference") (OtherActor :type "Actor Object Reference") (OtherComp :type "PrimitiveComponent Object Reference") (OtherBodyIndex :type Integer))
  (if (`KismetMathLibrary.ClassIsChildOf` (`GameplayStatics.GetObjectClass` OtherActor) "/Game/FirstPersonBP/Blueprints/FirstPersonCharacter.FirstPersonCharacter_C")
    (`SceneComponent.SetVisibility` (`self.Nameplate`) false false)
    (`self.DisableInput` (`GameplayStatics.GetPlayerController` 0))))

(event `Key|E`
  (params (Key :type "Key Structure"))
  (:`Pressed`
    (bind _successfullyadded (`/Game/GatheringSystem/Inventory/Libraries/BPFL_Inventory.Additem` (`self.Information`) (`.Quantity_17_3D2A65554277D23490ABBAA41E9C4759` (break `/Game/GatheringSystem/Inventory/Structures/ST_Item` (`self.Information`)))))
    (if _successfullyadded
      (`self.K2_DestroyActor`))))

(fn `UserConstructionScript`
  (bind (_datatable _rowname) (break `DataTableRowHandle` (`self.Item`)))
  ;[1 1 1] Get the ST_Item structure that corresponds with the row specified in the "item" variable, and assign it to our "information" variable
  (bind _returnvalue (`|GetDataTableRow` _datatable _rowname)
    (:`then`
      (set `self.Information` _returnvalue)
      ;[1 1 1] Update the mesh to whatever is defined in our "information" variable
      (`StaticMeshComponent.SetStaticMesh` (`self.Model`) (`.Model_14_F200B76E4885986D5143F39F95BC4A80` (break `/Game/GatheringSystem/Inventory/Structures/ST_Item` (`self.Information`)))))))