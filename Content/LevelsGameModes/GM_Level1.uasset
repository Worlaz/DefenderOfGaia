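; Level 1 game mode that runs enemy waves with a countdown and opens the game-over level when player or map health runs out.
; Tick updates the remaining NPC count, checks defeat, and uses Delays to alternate between countdown-then-spawn and advancing the wave once no enemies remain.
; SpawnEnemies places regular and heavy NPCs across SpawnPoints, handing each the first Path actor.
; A looping timer drives the countdown value; the final wave only prints a win message.
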(event `self.ReceiveBeginPlay`
  ;[1 1 1] ADD TO FIRSTPERSONCHARACTER
  (bind _returnvalue (`|CreateWidget` "/Game/LevelsGameModes/WG_DisplayCountDown.WG_DisplayCountDown_C"))
  (`UserWidget.AddToViewport` _returnvalue 0)
  (`Widget.SetVisibility` _returnvalue "Hidden")
  (bind _returnvalue_2 (`|CreateWidget` "/Game/LevelsGameModes/WG_Display_MapHealth.WG_Display_MapHealth_C"))
  (`UserWidget.AddToViewport` _returnvalue_2 0))

(event `self.ReceiveTick`
  (params (DeltaSeconds :type "Float (single-precision)"))
  (bind _countdowntime (`self.CountDownTime`))
  (bind _enemies (`self.GetRemainingNPCs`))
  (set `self.RemainingNPCs` _enemies)
  (bind _dead (`self.AreWeDead`))
  (if _dead
    (`KismetSystemLibrary.PrintString` "GAME OVER")
    (`GameplayStatics.OpenLevel` "GameOver_level")
    (else
      (`KismetSystemLibrary.Delay` 1.0)
      (if (`self.WaveInProgress`)
        (`KismetSystemLibrary.Delay` (`self.CountDownTime`))
        (bind _dead_2 (`self.EnemiesDead`))
        (if _dead_2
          (set `self.WaveInProgress` false)
          (set `self.CurrentWave` (+ (`self.CurrentWave`) 1)))
        (else
          (set `self.WaveInProgress` true)
          (`Widget.SetVisibility` (stale `self.ReceiveBeginPlay` _returnvalue) "Visible")
          (`self.CountDown` _countdowntime)
          (`KismetSystemLibrary.Delay` _countdowntime)
          (`Widget.SetVisibility` (stale `self.ReceiveBeginPlay` _returnvalue) "Hidden")
          (switch `int` (`self.CurrentWave`)
            (:`0`
              (`self.Spawn_Enemies` 1 1))
            (:`1`
              (`self.Spawn_Enemies` 0 1))
            (:`2`
              (`KismetSystemLibrary.PrintString` "YOU WONNED"))))))))

(fn `AreWeDead`
  (returns (Dead :type Boolean))
  (bind _asfirst_person_character (cast `/Game/FirstPersonBP/Blueprints/FirstPersonCharacter` (`GameplayStatics.GetPlayerCharacter` 0)))
  (if (<= (`/Game/FirstPersonBP/Blueprints/FirstPersonCharacter.CurrentHealth` _asfirst_person_character) 0.0)
    (`KismetSystemLibrary.PrintString` "Player died")
    (return true)
    (elif (<= (`self.MapHealth`) 0.0)
      (`KismetSystemLibrary.PrintString` "Died to NPSs coming through")
      (return true)
      (else
        (return false)))))

(fn `CountDown`
  (params (Time :type "Float (double-precision)"))
  (set `self.CountDownRemaining` Time)
  (`KismetSystemLibrary.K2_SetTimer` null "TimerCount" 1.0 true)
  (return))

(fn `EnemiesDead`
  (returns (Dead :type Boolean))
  (bind _outactors (`GameplayStatics.GetAllActorsOfClass` "/Game/AI/NPC/ModifiedNPC/BP_Parent_Enemy_NPC.BP_Parent_Enemy_NPC_C"))
  (`/Engine/EditorBlueprintResources/StandardMacros.IsValid` (`|GetArrayItem` _outactors)
    (:`Is Valid`
      (return false))
    (:`Is Not Valid`
      (return true))))

(fn `GetRemainingNPCs`
  (returns (Enemies :type Integer))
  (bind _outactors (`GameplayStatics.GetAllActorsOfClass` "/Game/AI/NPC/ModifiedNPC/BP_Parent_Enemy_NPC.BP_Parent_Enemy_NPC_C"))
  (return (`KismetArrayLibrary.Array_Length` _outactors)))

(fn `Spawn_Enemies`
  (params (Regular_NPC :type Integer) (Heavy_NPC :type Integer))
  (`|ExecutionSequence`
    (:`then_0`
      (set `self.Spawn_Index` 0)
      (bind _outactors (`GameplayStatics.GetAllActorsOfClass` "/Game/AI/NPC/Pathfinding/Path.Path_C"))
      (bind _output (`|GetArrayItem` _outactors))
      (`/Engine/EditorBlueprintResources/StandardMacros.IsValid` _output
        (:`Is Valid`
          (for _ (range 1 (+ Regular_NPC 1))
            (`|SpawnActorFromClass` "/Game/AI/NPC/ModifiedNPC/BP_Regular_Enemy_NPC.BP_Regular_Enemy_NPC_C" (`|GetArrayItem` (`self.Spawn_Points`) (`self.Spawn_Index`)) "Undefined" "OverrideRootScale" null _output null)
            (`KismetSystemLibrary.PrintString` "Spawned one")
            (if (< (`self.Spawn_Index`) (`KismetArrayLibrary.Array_Length` (`self.Spawn_Points`)))
              (set `self.Spawn_Index` (+ (`self.Spawn_Index`) 1))
              (else
                (set `self.Spawn_Index` 0)))))
        (:`Is Not Valid`
          (`KismetSystemLibrary.PrintString` "NO VALID PATH"))))
    (:`then_1`
      (set `self.Spawn_Index` 0)
      (bind _outactors_2 (`GameplayStatics.GetAllActorsOfClass` "/Game/AI/NPC/Pathfinding/Path.Path_C"))
      (bind _output_2 (`|GetArrayItem` _outactors_2))
      (`/Engine/EditorBlueprintResources/StandardMacros.IsValid` _output_2
        (:`Is Valid`
          (for _ (range 1 (+ Heavy_NPC 1))
            (`|SpawnActorFromClass` "/Game/AI/NPC/ModifiedNPC/BP_Heavy_Enemy_NPC.BP_Heavy_Enemy_NPC_C" (`|GetArrayItem` (`self.Spawn_Points`) (`self.Spawn_Index`)) "Undefined" "OverrideRootScale" null _output_2 null)
            (`KismetSystemLibrary.PrintString` "Spawned one")
            (if (< (`self.Spawn_Index`) (`KismetArrayLibrary.Array_Length` (`self.Spawn_Points`)))
              (set `self.Spawn_Index` (+ (`self.Spawn_Index`) 1))
              (else
                (set `self.Spawn_Index` 0)))))
        (:`Is Not Valid`
          (`KismetSystemLibrary.PrintString` "NO VALID PATH"))))))

(fn `TimerCount`
  (bind _output_get (set `self.CountDownRemaining` (- (`self.CountDownRemaining`) 1.0)))
  (if (<= _output_get 0.0)
    (`KismetSystemLibrary.K2_ClearTimer` null "TimerCount")))

(fn `UserConstructionScript`)